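; Enemy turret that tracks the player pawn and fires twin barrels while the player is within attack range.
; Each tick updates the range flag, then interpolates gantry yaw and gun rotation with clamped pitch.
; Firing is requested every tick, with a Delay throttling bullet spawns from two gun sockets.
; TakeDamage subtracts fixed health and prints it, with no death handling.
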(event `self.ReceiveTick`
  (params (DeltaSeconds :type "Float (single-precision)"))
  (set `self.DeltaTime` DeltaSeconds)
  (`self.Update Range`)
  (`self.Update Rotation`)
  (`self.FireWeapons`))

(event `Update Rotation`
  (if (`self.EnemyInRange`)
    ;[1 1 1] Setting The Gantry's Rotation
    (`SceneComponent.K2_SetWorldRotation` (`self.Gantry`) (`KismetMathLibrary.RInterpTo` (`SceneComponent.K2_GetComponentRotation` (`self.Gantry`)) (`KismetMathLibrary.MakeRotator` 0.0 0.0 (.yaw (`KismetMathLibrary.FindLookAtRotation` (`SceneComponent.K2_GetComponentLocation` (`self.Gantry`)) (`self.K2_GetActorLocation` (`GameplayStatics.GetPlayerPawn` 0))))) (`self.DeltaTime`) (`self.RotationSpeed`)) false false)
    ;[1 1 1] Setting the Turret's Guns Rotation
    (`SceneComponent.K2_SetWorldRotation` (`self.Guns`) (`KismetMathLibrary.RInterpTo` (`SceneComponent.K2_GetComponentRotation` (`self.Guns`)) (`KismetMathLibrary.MakeRotator` 0.0 (`KismetMathLibrary.ClampAngle` (- (.pitch (`KismetMathLibrary.FindLookAtRotation` (`SceneComponent.K2_GetComponentLocation` (`self.Guns`)) (`self.K2_GetActorLocation` (`GameplayStatics.GetPlayerPawn` 0)))) (`self.BarrelLength`)) -10.0 35.0) (.yaw (`KismetMathLibrary.FindLookAtRotation` (`SceneComponent.K2_GetComponentLocation` (`self.Guns`)) (`self.K2_GetActorLocation` (`GameplayStatics.GetPlayerPawn` 0))))) (`self.DeltaTime`) (`self.RotationSpeed`)) false false)
    (`self.FireWeapons`)))

(event `FireWeapons`
  (bind _guns (`self.Guns`))
  ;[1 1 1] Fire Weapons
  (if (`self.EnemyInRange`)
    (`KismetSystemLibrary.Delay` (`self.FireInterval`))
    (`|SpawnActorFromClass` "/Game/VehicleAdvBP/Blueprints/Bullet.Bullet_C" (`SceneComponent.GetSocketTransform` _guns "Barrel_1" "RTS_World") "Undefined" "OverrideRootScale")
    (`|SpawnActorFromClass` "/Game/VehicleAdvBP/Blueprints/Bullet.Bullet_C" (`SceneComponent.GetSocketTransform` _guns "Barrel_2" "RTS_World") "Undefined" "OverrideRootScale")))

(event `Update Range`
  ;[1 1 1] If enemy is within site, change the bool to true
  (if (<= (`self.GetDistanceTo` (`GameplayStatics.GetPlayerPawn` 0)) (`self.AttackRange`))
    (set `self.EnemyInRange` true)
    (else
      (set `self.EnemyInRange` false))))

(fn `TakeDamage`
  (set `self.EnemyHealth` (- (`self.EnemyHealth`) 5))
  (`KismetSystemLibrary.PrintString` (`KismetStringLibrary.Concat_StrStr` "Current health:" (`KismetStringLibrary.Conv_IntToString` (`self.EnemyHealth`)))))

(fn `UserConstructionScript`)