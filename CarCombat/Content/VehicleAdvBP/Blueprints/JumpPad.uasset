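; Jump pad actor that launches the player's vehicle upward while it is active.
; On Tick, a Delay gates a random roll every few seconds that switches the pad on or off.
; A dynamic material created in the construction script turns the cube red when active and white when inactive.
; Any actor overlap while active applies a large vertical impulse to player zero's VehicleBlueprint mesh, without checking what overlapped.
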(event `self.ReceiveActorBeginOverlap`
  (params (OtherActor :type "Actor Object Reference"))
  (if (`self.isActive`)
    (`self.Launch Player`)))

(event `self.ReceiveTick`
  (params (DeltaSeconds :type "Float (single-precision)"))
  ;[1 1 1] Activating the Launchpad at random interval, for a random amount of time
  (`KismetSystemLibrary.Delay` (`KismetMathLibrary.RandomFloatInRange` 1.0 3.0))
  (`/Engine/EditorBlueprintResources/StandardMacros.CompareInt` (`KismetMathLibrary.RandomIntegerInRange` 1 10) 5
    (:`>`
      ;[1 1 1] Changing the colour to red when active to notfiy player
      (set `self.isActive` true)
      (`MaterialInstanceDynamic.SetVectorParameterValue` (`self.DynMat`) "Color" (make `LinearColor` 255.0 0.0 0.0 1.0)))
    (:`<`
      ;[1 1 1] Changing the colour back to white when inactive
      (set `self.isActive` false)
      (`MaterialInstanceDynamic.SetVectorParameterValue` (`self.DynMat`) "Color" (make `LinearColor` 1.0 1.0 1.0 1.0)))))

(fn `Launch Player`
  (bind _asvehicle_blueprint (cast `/Game/VehicleAdvBP/Blueprints/VehicleBlueprint` (`GameplayStatics.GetPlayerPawn` 0)))
  (`PrimitiveComponent.AddImpulse` (`WheeledVehicle.Mesh` _asvehicle_blueprint) (0.0 0.0 2000000.0) "None" false))

(fn `UserConstructionScript`
  (bind _returnvalue (`PrimitiveComponent.CreateDynamicMaterialInstance` (`self.Cube`) 0 null))
  (set `self.DynMat` _returnvalue))