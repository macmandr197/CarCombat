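; Bullet projectile actor that damages the player's vehicle when it hits it.
; On Hit, it checks for player pawn 0, casts it to VehicleBlueprint, calls TakeDamage and destroys itself; other hits are ignored.
; Any actor overlap prints the other actor's name and destroys the bullet without dealing damage.
; The static mesh's overlap event and the construction script are empty.
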(event `self.ReceiveHit`
  (params (MyComp :type "PrimitiveComponent Object Reference") (Other :type "Actor Object Reference") (OtherComp :type "PrimitiveComponent Object Reference") (bSelfMoved :type Boolean) (HitLocation :type "Vector Structure") (HitNormal :type "Vector Structure") (NormalImpulse :type "Vector Structure") (Hit :type "HitResult Structure (by ref)"))
  (if (== Other (`GameplayStatics.GetPlayerPawn` 0))
    (bind _asvehicle_blueprint (cast `/Game/VehicleAdvBP/Blueprints/VehicleBlueprint` (`GameplayStatics.GetPlayerPawn` 0)))
    (`/Game/VehicleAdvBP/Blueprints/VehicleBlueprint.TakeDamage` _asvehicle_blueprint)
    (`self.K2_DestroyActor`)))

(event `self.StaticMesh.OnComponentBeginOverlap`
  (params (OverlappedComponent :type "PrimitiveComponent Object Reference") (OtherActor :type "Actor Object Reference") (OtherComp :type "PrimitiveComponent Object Reference") (OtherBodyIndex :type Integer) (bFromSweep :type Boolean) (SweepResult :type "HitResult Structure (by ref)")))

(event `self.ReceiveActorBeginOverlap`
  (params (OtherActor :type "Actor Object Reference"))
  (`KismetSystemLibrary.PrintString` (`KismetSystemLibrary.GetDisplayName` (stale `self.ReceiveHit` Other)))
  (`self.K2_DestroyActor`))

(fn `UserConstructionScript`)