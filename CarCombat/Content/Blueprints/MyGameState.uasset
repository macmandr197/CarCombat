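; MyGameState is a game state Blueprint that runs a match countdown and ends the game when time runs out.
; On BeginPlay, only the server starts a looping one-second timer that decrements CountDownTime.
; At zero it casts player 0's pawn to VehicleBlueprint, destroys it, sets IsGameOver and clears the timer.
; If that cast fails, game over is not set and the timer keeps running.
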(event `self.ReceiveBeginPlay`
  ;[1 1 1] Set Timer
  (if (`KismetSystemLibrary.IsServer`)
    (`KismetSystemLibrary.K2_SetTimer` null "Timer/Count" 1.0 true)))

(event `Timer/Count`
  ;[1 1 1] Countdown function
  (bind _output_get (set `self.CountDownTime` (- (`self.CountDownTime`) 1.0)))
  (if (<= _output_get 0.0)
    (bind _asvehicle_blueprint (cast `/Game/Blueprints/Player/VehicleBlueprint` (`GameplayStatics.GetPlayerPawn` 0)))
    (`self.K2_DestroyActor` _asvehicle_blueprint)
    (set `self.isGameOver` true)
    (`KismetSystemLibrary.K2_ClearTimer` null "Timer/Count")))

(fn `NewFunction_0`)

(fn `UserConstructionScript`)